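; BP_Ball is a menu animation Blueprint for a ball that advances along a list of target points each time its sphere is overlapped.
; Sphere1's begin-overlap fires BallMovement, which uses MoveComponentTo to move the root component toward the indexed target actor's location over a per-step duration.
; It then increments the index and calls ControlMovedol, whose body is not shown here.
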(event OnComponentBeginOverlap(Sphere1)
  (params (OverlappedComponent :type Primitive%20Component%20Object%20Reference) (OtherActor :type Actor%20Object%20Reference) (OtherComp :type Primitive%20Component%20Object%20Reference) (OtherBodyIndex :type Integer) (bFromSweep :type Boolean) (SweepResult :type Hit%20Result%20Structure%20%28by%20ref%29))
  (CallFunction|BallMovement))

(event Custom|BallMovement
  (Components|MoveComponentTo (Variables|Default|GetDefaultSceneRoot) (Transformation|GetActorLocation (Utilities|Array|Get(acopy) (Variables|Default|GetTarget) (Variables|Default|Getindex))) "0, 0, 0" false false (Utilities|Array|Get(acopy) (Variables|Default|GetOver%20Time) (Variables|Default|Getindex)) false)
  (bind _result (Math|Integer|IncrementInt (Variables|Default|Getindex))
    (:%20%20
      (Variables|Default|Setindex _result)
      (CallFunction|ControlMovedol))))

(fn ConstructionScript)