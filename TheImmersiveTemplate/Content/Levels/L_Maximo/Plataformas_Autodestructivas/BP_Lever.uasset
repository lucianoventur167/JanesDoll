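; BP_Lever is a lever actor that switches the movement of every BP_Platform in the level while a Character stands within its sphere.
; BeginPlay makes the sphere visible in game and caches all platform actors.
; Each Tick polls the sphere for an overlapping Character, sets LeverOn accordingly, and copies it to every platform's Movement flag, so the lever acts as a hold switch rather than a toggle.
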(event EventBeginPlay
  (Development|SetHiddeninGame (Variables|Default|GetSphere) false false)
  (bind _outactors (Actor|GetAllActorsOfClass "/Game/Levels/L_Maximo/Plataformas_Autodestructivas/BP_Platform.BP_Platform_C")))

(event Collision|EventActorBeginOverlap
  (params (OtherActor :type Actor%20Object%20Reference)))

(event EventTick
  (params (DeltaSeconds :type Float%20%28single-precision%29))
  (if (Utilities|IsValid (Utilities|Array|Get(acopy) (Collision|GetOverlappingActors (Variables|Default|GetSphere) "/Script/Engine.Character" :!class /Script/Engine.PrimitiveComponent)))
    (Variables|Default|SetLever_on? true)
    (else
      (Variables|Default|SetLever_on? false)))
  (for _array_element (stale EventBeginPlay _outactors)
    (Variables|/Game/Levels/L_Maximo/Plataformas_Autodestructivas/BP_Platform.BP_Platform_C|SetMovement? _array_element (Variables|Default|GetLever_on?))))

(fn ConstructionScript)