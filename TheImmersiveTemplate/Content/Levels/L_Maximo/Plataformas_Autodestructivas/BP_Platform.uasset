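; Self-destructing platform that vanishes after something overlaps its Box trigger, then reappears.
; The overlap waits TiempoDeDestruccion, hides Platform and disables its collision, then after TiempoDeReaparicion shows it with QueryAndProbe collision.
; Tick polls the Movement flag, using two DoOnce nodes that reset each other to stop or restart InterpToMovement once per change.
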(event OnComponentBeginOverlap(Box)
  (params (OverlappedComponent :type Primitive%20Component%20Object%20Reference) (OtherActor :type Actor%20Object%20Reference) (OtherComp :type Primitive%20Component%20Object%20Reference) (OtherBodyIndex :type Integer) (bFromSweep :type Boolean) (SweepResult :type Hit%20Result%20Structure%20%28by%20ref%29))
  (bind _platform (Variables|Default|GetPlatform))
  (bind _platform_2 (Variables|Default|GetPlatform))
  (Utilities|FlowControl|Delay (Variables|Default|GetTiempo%20de%20destruccion))
  (Development|SetHiddeninGame _platform_2 true true)
  (Collision|SetCollisionEnabled _platform_2 "NoCollision")
  (Utilities|FlowControl|Delay (Variables|Default|GetTiempo%20de%20reaparicion))
  (Development|SetHiddeninGame _platform false true)
  (Collision|SetCollisionEnabled _platform "QueryAndProbe")
  (Development|SetHiddeninGame (Variables|Default|GetBox) true false))

(event EventTick
  (params (DeltaSeconds :type Float%20%28single-precision%29))
  (if (not (Variables|Default|GetMovement?))
    (Utilities|FlowControl|DoOnce false :!label _label
      (:Completed
        (Components|Movement|StopMovementImmediately (Variables|Default|GetInterpToMovement))
        (goto _label_2 Reset)))
    (else
      (Utilities|FlowControl|DoOnce false :!label _label_2
        (:Completed
          (Class|InterptoMovementComponent|RestartMovement (Variables|Default|GetInterpToMovement) 1.0)
          (goto _label Reset))))))

(fn ConstructionScript)