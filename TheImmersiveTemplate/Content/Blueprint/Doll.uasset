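; Doll Blueprint that continuously animates its static mesh up and down along the Z axis from BeginPlay.
; A Timeline track drives the mesh's relative Z location on each update.
; The custom Animation event toggles a boolean to play or reverse the Timeline, and the Timeline's Finished output calls it again, forming a ping-pong loop without Tick.
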(event Custom|Animation
  (if (not (Variables|Default|Getanim))
    (Variables|Default|Setanim true)
    (bind _newtrack_0 (Timeline|Timeline Play)
      (:Update
        (Transformation|SetRelativeLocation (Variables|Default|GetStaticMesh) (Math|Vector|MakeVector 0.0 0.0 _newtrack_0) false false))
      (:Finished
        (CallFunction|Animation)))
    (else
      (Variables|Default|Setanim false)
      (Timeline|Timeline Reverse))))

(event EventBeginPlay
  (CallFunction|Animation))

(fn ConstructionScript)