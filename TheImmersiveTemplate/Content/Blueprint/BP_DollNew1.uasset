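; BP_DollNew1 is a doll actor that animates in place, then travels away and vanishes when the player reaches it.
; From BeginPlay, a Timeline alternates between play and reverse on a flag to bob the static mesh along Z.
; When BP_ImmersiveCharacter overlaps the box, chained MoveComponentTo calls carry the root through three target actors' locations before the doll destroys itself, with debug prints along the way.
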(event OnComponentBeginOverlap(Box)
  (params (OverlappedComponent :type Primitive%20Component%20Object%20Reference) (OtherActor :type Actor%20Object%20Reference) (OtherComp :type Primitive%20Component%20Object%20Reference) (OtherBodyIndex :type Integer) (bFromSweep :type Boolean) (SweepResult :type Hit%20Result%20Structure%20%28by%20ref%29))
  ;[1 1 1] Collision
  (Development|PrintString "Hello")
  (Utilities|Casting|CastToBP_ImmersiveCharacter OtherActor)
  (Development|PrintString "move")
  (CallFunction|MoveDoll1))

(event Custom|Animación
  ;[1 1 1] Animacion Muñeca
  (if (not (Variables|Default|GetAnim1))
    (Variables|Default|SetAnim1 true)
    (bind _newtrack_0 (Timeline|Timeline Play)
      (:Update
        (Transformation|SetRelativeLocation (Variables|Default|GetStaticMesh) (Math|Vector|MakeVector 0.0 0.0 _newtrack_0) false false))
      (:Finished
        (CallFunction|Animación)))
    (else
      (Variables|Default|SetAnim1 false)
      (Timeline|Timeline Reverse))))

(event Custom|MoveDoll1
  ;[1 1 1] Movimiento
  (Components|MoveComponentTo (Variables|Default|GetDefaultSceneRoot) (Transformation|GetActorLocation (Variables|Default|GetTarget%20Actor)) "0, 0, 0" false false 3.0 false)
  (Development|PrintString "termino")
  (Components|MoveComponentTo (Variables|Default|GetDefaultSceneRoot) (Transformation|GetActorLocation (Variables|Default|GetTarget%20Actor2)) "0, 0, 0" false false 1.0 false)
  (Components|MoveComponentTo (Variables|Default|GetDefaultSceneRoot) (Transformation|GetActorLocation (Variables|Default|GetTarget%20Actor3)) "0, 0, 0" false false 1.0 false)
  (Actor|DestroyActor))

(event EventBeginPlay
  (CallFunction|Animación))

(fn ConstructionScript)