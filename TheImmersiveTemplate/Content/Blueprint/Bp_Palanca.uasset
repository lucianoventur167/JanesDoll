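; Lever actor that sets a group of platforms moving.
; Its box overlap stores the lever as the Palanca reference on the third-person character and clears it when the overlap ends.
; The MovePlataforme event calls the event of the same name on each entry in the Plataformas array, re-invoking itself with an incrementing index that resets to zero after the last one.
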(event OnComponentBeginOverlap(Box)
  (params (OverlappedComponent :type Primitive%20Component%20Object%20Reference) (OtherActor :type Actor%20Object%20Reference) (OtherComp :type Primitive%20Component%20Object%20Reference) (OtherBodyIndex :type Integer) (bFromSweep :type Boolean) (SweepResult :type Hit%20Result%20Structure%20%28by%20ref%29))
  (bind _asbp_third_person_character (Utilities|Casting|CastToBP_ThirdPersonCharacter OtherActor))
  (Variables|/Game/ThirdPerson/Blueprints/BP_ThirdPersonCharacter.BP_ThirdPersonCharacter_C|SetPalanca _asbp_third_person_character self))

(event OnComponentEndOverlap(Box)
  (params (OverlappedComponent :type Primitive%20Component%20Object%20Reference) (OtherActor :type Actor%20Object%20Reference) (OtherComp :type Primitive%20Component%20Object%20Reference) (OtherBodyIndex :type Integer))
  (bind _asbp_third_person_character (Utilities|Casting|CastToBP_ThirdPersonCharacter OtherActor))
  (Variables|/Game/ThirdPerson/Blueprints/BP_ThirdPersonCharacter.BP_ThirdPersonCharacter_C|SetPalanca _asbp_third_person_character 0))

(event Custom|MovePlataforme
  (Default|MovePlataforme (Utilities|Array|Get(acopy) (Variables|Default|GetPlataformas) (Variables|Default|Getindex)))
  (bind _result (Math|Integer|IncrementInt (Variables|Default|Getindex))
    (:%20%20
      (Variables|Default|Setindex _result)
      (if (== (Utilities|Array|Length (Variables|Default|GetPlataformas)) (Variables|Default|Getindex))
        (Variables|Default|Setindex 0)
        (else
          (CallFunction|MovePlataforme))))))

(fn ConstructionScript)