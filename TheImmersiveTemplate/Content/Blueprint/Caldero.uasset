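; Cauldron Blueprint (Caldero) that consumes pickup boxes overlapping its Box collision and counts them.
; The first box starts a self-calling one-second Delay countdown on Time, which resets Time to 10 and clears the count when it reaches zero.
; Each pickup prints the count and runs a completion check that currently only prints to screen when exactly one object is counted.
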(event OnComponentBeginOverlap(Box)
  (params (OverlappedComponent :type Primitive%20Component%20Object%20Reference) (OtherActor :type Actor%20Object%20Reference) (OtherComp :type Primitive%20Component%20Object%20Reference) (OtherBodyIndex :type Integer) (bFromSweep :type Boolean) (SweepResult :type Hit%20Result%20Structure%20%28by%20ref%29))
  (bind _asbp_object_pickup_box (Utilities|Casting|CastToBP_Object_Pickup_Box OtherActor))
  (if (== (Variables|Default|GetObjects) 0)
    (CallFunction|Timer))
  (Actor|DestroyActor _asbp_object_pickup_box)
  (bind _result (Math|Integer|IncrementInt (Variables|Default|GetObjects))
    (:%20%20
      (bind _output_get (Variables|Default|SetObjects _result))
      (Development|PrintString (Utilities|String|ToString(Integer) _output_get))
      (CallFunction|IsCompleteEvent))))

(event Custom|Timer
  (Utilities|FlowControl|Delay 1.0)
  (bind _result (Math|Integer|DecrementInt (Variables|Default|GetTime))
    (:%20%20
      (if (== _result 0)
        (Variables|Default|SetTime 10)
        (Variables|Default|SetObjects 0)
        (else
          (CallFunction|Timer))))))

(event Custom|IsCompleteEvent
  (bind _objects (Variables|Default|GetObjects))
  (bind _returnvalue (== _objects 1))
  (Development|PrintString (Utilities|String|ToString(Boolean) _returnvalue) _returnvalue))

(fn ConstructionScript)