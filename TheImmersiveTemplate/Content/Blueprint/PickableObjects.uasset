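; PickableObjects is an object the third-person character can pick up.
; When the character overlaps its Box while picking up, it disables physics simulation and collision on both the static mesh and the box.
; Its Interact function prints a Spanish debug message ("Agarra el objeto") and returns the mesh asset to the caller; the Blueprint itself does no attaching.
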(event OnComponentBeginOverlap(Box)
  (params (OverlappedComponent :type Primitive%20Component%20Object%20Reference) (OtherActor :type Actor%20Object%20Reference) (OtherComp :type Primitive%20Component%20Object%20Reference) (OtherBodyIndex :type Integer) (bFromSweep :type Boolean) (SweepResult :type Hit%20Result%20Structure%20%28by%20ref%29))
  (Utilities|Casting|CastToBP_ThirdPersonCharacter OtherActor)
  (Utilities|IsValid 0
    (:Is%20Valid
      (if (Variables|/Game/ThirdPerson/Blueprints/BP_ThirdPersonCharacter.BP_ThirdPersonCharacter_C|GetIsPickingUp (Variables|Default|GetPlayer))
        (Physics|SetSimulatePhysics (Variables|Default|GetStaticMesh) false)
        (Collision|SetCollisionEnabled (Variables|Default|GetStaticMesh) "NoCollision")))))

(fn ConstructionScript)

(fn Interact
  (Development|PrintString "Agarra el objeto")
  (return (Variables|/Script/Engine.StaticMeshComponent|GetStaticMesh (Variables|Default|GetStaticMesh))))